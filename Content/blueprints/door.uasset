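; Door actor Blueprint that the player toggles open and closed with the E key while inside its Box trigger.
; Box overlap begin and end enable and disable input for player controller 0, without filtering the overlapping actor.
; E plays Collapse01 at the world origin, then flips DoorClosed and plays or reverses the Dooropenclose timeline.
; The timeline lerps the Door's world yaw between 0 and 90 degrees.
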(event OnComponentBeginOverlap(Box)
  (params (OverlappedComponent :type Primitive%20Component%20Object%20Reference) (OtherActor :type Actor%20Object%20Reference) (OtherComp :type Primitive%20Component%20Object%20Reference) (OtherBodyIndex :type Integer) (bFromSweep :type Boolean) (SweepResult :type Hit%20Result%20Structure%20%28by%20ref%29))
  ;[1 1 1] enable/disable input
  (Input|EnableInput (Game|GetPlayerController 0)))

(event OnComponentEndOverlap(Box)
  (params (OverlappedComponent :type Primitive%20Component%20Object%20Reference) (OtherActor :type Actor%20Object%20Reference) (OtherComp :type Primitive%20Component%20Object%20Reference) (OtherBodyIndex :type Integer))
  ;[1 1 1] enable/disable input
  (Input|DisableInput (Game|GetPlayerController 0)))

(event EventBeginPlay)

(event Collision|EventActorBeginOverlap
  (params (OtherActor :type Actor%20Object%20Reference)))

(event EventTick
  (params (DeltaSeconds :type Float%20%28single-precision%29)))

(event Input|KeyboardEvents|E
  (params (Key :type Key%20Structure :default "None"))
  ;[1 1 1] open/close
  (:Pressed
    (Audio|PlaySoundatLocation "/Game/StarterContent/Audio/Collapse01.Collapse01" "0, 0, 0" "0, 0, 0" 1.0 1.0 0.0 0 0 0)
    (if (Variables|Default|Getdoor_closed)
      (Variables|Default|Setdoor_closed false)
      (bind _open_close (Timeline|dooropen/close Play)
        (:Update
          (Transformation|SetWorldRotation (Variables|Default|Getdoor) (Math|Rotator|MakeRotator 0.0 0.0 (Math|Float|Lerp 0.0 9e+01 _open_close)) false false)))
      (else
        (Variables|Default|Setdoor_closed true)
        (Timeline|dooropen/close Reverse)))))

(fn ConstructionScript)